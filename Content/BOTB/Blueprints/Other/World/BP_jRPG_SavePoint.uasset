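; BP_jRPG_SavePoint is a world save point that activates when the player character enters its radius.
; Overlap registers it as SavePointReference on the player controller's AC_jRPG_SaveManager and clears that on exit; saving itself is not handled here.
; While the player is inside, looping timelines spin and bob the cube, a scale timeline pops up the text, and Tick smoothly yaws that text toward the player.
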(event `self.ReceiveTick`
  (params (DeltaSeconds :type "Float (single-precision)"))
  (bind _textrenderingame (`self.TextRenderInGame`))
  ;[1 1 1] Rotates text toward player.
  (bind _focusactor (`self.FocusActor`)
    (:`then`
      (bind (_returnvalue_roll _returnvalue_pitch _returnvalue_yaw) (`KismetMathLibrary.BreakRotator` (`KismetMathLibrary.RInterpTo` (`SceneComponent.K2_GetComponentRotation` _textrenderingame) (`KismetMathLibrary.FindLookAtRotation` (`SceneComponent.K2_GetComponentLocation` _textrenderingame) (`self.K2_GetActorLocation` _focusactor)) (`GameplayStatics.GetWorldDeltaSeconds`) 10.0)))
      (`SceneComponent.K2_SetWorldRotation` (`self.TextRenderInGame`) (`KismetMathLibrary.MakeRotator` 0.0 0.0 _returnvalue_yaw) false false))
    (:`else`)))

(event `RotateCube`
  ;[1 1 1] Cube floating and rotation.
  (bind (_direction _yaw _locz) (`Timeline|Timeline_CubeRotator` :!label _label)
    (:`Update`
      (`SceneComponent.K2_SetRelativeRotation` (`self.Cube`) (`KismetMathLibrary.MakeRotator` -55.0 30.0 _yaw) false false)
      (`SceneComponent.K2_SetRelativeLocation` (`self.Cube`) (`KismetMathLibrary.MakeVector` 0.0 0.0 _locz) false false))
    (:`Finished`
      (`KismetSystemLibrary.Delay` 0.05)
      (goto _label :!via `PlayFromStart`))))

(event `StopCube`
  (goto _label :!via `Stop`))

(event `ShowText`
  ;[1 1 1] Pop up or hide text
  (bind (_direction _textscale) (`Timeline|Timeline_ShowText` :!label _label_2)
    (:`Update`
      (`SceneComponent.SetRelativeScale3D` (`self.TextRenderInGame`) (* (1.0 1.0 1.0) _textscale)))))

(event `HideText`
  ;[1 1 1] Pop up or hide text
  (goto _label_2 :!via `Reverse`))

(event `self.ActivationRadius.OnComponentBeginOverlap`
  (params (OverlappedComponent :type "PrimitiveComponent Object Reference") (OtherActor :type "Actor Object Reference") (OtherComp :type "PrimitiveComponent Object Reference") (OtherBodyIndex :type Integer) (bFromSweep :type Boolean) (SweepResult :type "HitResult Structure (by ref)"))
  (bind _returnvalue (`GameplayStatics.GetPlayerCharacter` 0))
  ;[1 1 1] Toggle save interaction when player is in the range.
  (if (== OtherActor _returnvalue)
    (`self.RotateCube`)
    (set `self.FocusActor` _returnvalue)
    (`self.ShowText`)
    (set `/Game/BOTB/Blueprints/Components/AC_jRPG_SaveManager.SavePointReference` self (`self.GetComponentByClass` (`GameplayStatics.GetPlayerController` 0) "/Game/BOTB/Blueprints/Components/AC_jRPG_SaveManager.AC_jRPG_SaveManager_C"))))

(event `self.ActivationRadius.OnComponentEndOverlap`
  (params (OverlappedComponent :type "PrimitiveComponent Object Reference") (OtherActor :type "Actor Object Reference") (OtherComp :type "PrimitiveComponent Object Reference") (OtherBodyIndex :type Integer))
  ;[1 1 1] Toggle save interaction when player is in the range.
  (if (== OtherActor (`GameplayStatics.GetPlayerCharacter` 0))
    (`self.StopCube`)
    (set `self.FocusActor` null)
    (`self.HideText`)
    (set `/Game/BOTB/Blueprints/Components/AC_jRPG_SaveManager.SavePointReference` null (`self.GetComponentByClass` (`GameplayStatics.GetPlayerController` 0) "/Game/BOTB/Blueprints/Components/AC_jRPG_SaveManager.AC_jRPG_SaveManager_C"))))

(fn `UserConstructionScript`)